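; Story 2 tree actor that displays an enlarged effect above itself and swaps it when hit correctly.
; BeginPlay spawns the effect at the current Num, and later respawns pick Num randomly from four.
; A damage handler, rebound every Tick, accepts any damage for index zero, otherwise damage equal to Num, then destroys and respawns the effect.
; Unconnected nodes hold text popups and a wolf AI move trigger.
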(event `makeEffect`
  (set `self.num` (`KismetMathLibrary.RandomInteger` 4))
  (bind _returnvalue (`|SpawnActorFromClass` (`|GetArrayItem` (`self.Effect_List`) (`self.num`)) (`self.GetTransform`) "Undefined" "OverrideRootScale" null null :!label _label))
  (bind _output_get (set `self.object` (`Actor.RootComponent` _returnvalue)))
  (`SceneComponent.SetWorldScale3D` _output_get (6.0 6.0 6.0))
  (`SceneComponent.K2_SetWorldLocation` _output_get (+ (`self.K2_GetActorLocation`) (0.0 0.0 150.0)) false false)
  (set `self.isFrist` true))

(event `self.ReceiveBeginPlay`
  (goto _label))

(event `self.ReceiveTick`
  (params (DeltaSeconds :type "Float (single-precision)"))
  (add `self.OnTakeAnyDamage` (delegate `OnTakeAnyDamage_Event`)))

(event `OnTakeAnyDamage_Event` :!signature `self.OnTakeAnyDamage`
  (params (DamagedActor :type "Actor Object Reference") (Damage :type "Float (single-precision)") (DamageType :type "DamageType Object Reference") (InstigatedBy :type "Controller Object Reference") (DamageCauser :type "Actor Object Reference"))
  (if (`self.isFrist`)
    (if (== (`self.num`) 0)
      (`self.K2_DestroyActor` (`ActorComponent.GetOwner` (`self.object`)) :!label _label_2)
      (set `self.isFrist` false)
      (`self.makeEffect`)
      (elif (== Damage (`self.num`))
        (goto _label_2)))))

(event `OnDestroyed_이벤트_0` :!signature `self.OnDestroyed`
  (params (DestroyedActor :type "Actor Object Reference"))
  (`KismetSystemLibrary.Delay` 2.0)
  (bind _returnvalue (`GameplayStatics.GetActorOfClass` "/Game/Tutorial_etc/tutorial_wolf/wolf_AIcontroller.wolf_AIcontroller_C"))
  (`/Game/Tutorial_etc/tutorial_wolf/wolf_AIcontroller.moveToTele` _returnvalue))

(fn `UserConstructionScript`)