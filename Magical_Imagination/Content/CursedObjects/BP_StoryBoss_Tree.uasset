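; Cursed story-boss tree that shows a large effect above itself, which damage can clear, triggering story text.
; BeginPlay spawns the EffectList entry at the current Num, while makeEffect randomizes it first.
; Damage clears the effect when Num is zero or equals the damage amount.
; Only the first clear prints text; later text and the wolf teleport-move hookup are unreachable behind the Index check.
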(event `makeEffect`
  (set `self.num` (`KismetMathLibrary.RandomInteger` 6))
  (bind _returnvalue (`|SpawnActorFromClass` (`|GetArrayItem` (`self.Effect_List`) (`self.num`)) (`self.GetTransform`) "Undefined" "OverrideRootScale" null null :!label _label))
  (bind _output_get (set `self.object` (`Actor.RootComponent` _returnvalue)))
  (`SceneComponent.SetWorldScale3D` _output_get (6.0 6.0 6.0))
  (`SceneComponent.K2_SetWorldLocation` _output_get (+ (`self.K2_GetActorLocation`) (0.0 0.0 150.0)) false false)
  (set `self.isFrist` true))

(event `self.ReceiveBeginPlay`
  (goto _label))

(event `self.ReceiveTick`
  (params (DeltaSeconds :type "Float (single-precision)"))
  (add `self.OnTakeAnyDamage` (delegate `OnTakeAnyDamage_Event`)))

(event `OnTakeAnyDamage_Event` :!signature `self.OnTakeAnyDamage`
  (params (DamagedActor :type "Actor Object Reference") (Damage :type "Float (single-precision)") (DamageType :type "DamageType Object Reference") (InstigatedBy :type "Controller Object Reference") (DamageCauser :type "Actor Object Reference"))
  (bind _index (`self.index`))
  (if (`self.isFrist`)
    (if (== (`self.num`) 0)
      (`self.K2_DestroyActor` (`ActorComponent.GetOwner` (`self.object`)) :!label _label_2)
      (set `self.isFrist` false)
      (if (< _index 1)
        (bind _returnvalue (`|SpawnActorFromClass` :`Class` "/Game/UI/BP_Text_Print_2.BP_Text_Print_2_C" :`SpawnTransform` (`KismetMathLibrary.MakeTransform` (-563.0 2371.0 287.0)) :`CollisionHandlingOverride` "Undefined" :`TransformScaleMethod` "OverrideRootScale" :`Instigator` null))
        (switch `int` _index
          (:`0`
            (set `/Game/UI/BP_Text_Print_2.Text` (`self.Text_3_2`) _returnvalue))
          (:`1`
            (set `/Game/UI/BP_Text_Print_2.Text` (`self.Text_3_3`) _returnvalue))
          (:`2`
            (add `self.OnDestroyed` _returnvalue (delegate `OnDestroyed_이벤트_0`))
            (set `/Game/UI/BP_Text_Print_2.Text` (`self.Text_3_4`) _returnvalue)))
        (set `/Game/UI/BP_Text_Print_2.StartPlayDelay` 1.0 _returnvalue))
      (set `self.index` (+ (`self.index`) 1))
      (elif (== Damage (`self.num`))
        (goto _label_2)))))

(event `OnDestroyed_이벤트_0` :!signature `self.OnDestroyed`
  (params (DestroyedActor :type "Actor Object Reference"))
  (`KismetSystemLibrary.Delay` 2.0)
  (bind _returnvalue (`GameplayStatics.GetActorOfClass` "/Game/Tutorial_etc/tutorial_wolf/wolf_AIcontroller.wolf_AIcontroller_C"))
  (`/Game/Tutorial_etc/tutorial_wolf/wolf_AIcontroller.moveToTele` _returnvalue))

(fn `UserConstructionScript`)