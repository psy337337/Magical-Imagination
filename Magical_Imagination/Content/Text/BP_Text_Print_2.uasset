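; Trigger actor that plays a sequence of text lines on the VRPawn's text bar while blocking teleportation.
; It starts when the pawn enters its box, or after a BeginPlay delay if StartPlay is set.
; Tick offers the current line to ActiveTextBar, advancing when accepted, then restores teleporting and destroys the actor after the last.
; Any end overlap pauses it, as that actor check compares OtherActor to itself.
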(event `self.ReceiveTick`
  (params (DeltaSeconds :type "Float (single-precision)"))
  (bind _textindex (`self.TextIndex`))
  (if (`self.IsPlayerOn`)
    (if (> (`KismetArrayLibrary.Array_Length` (`self.Text`)) _textindex)
      (bind _iswrite (`/Game/VRTemplate/Blueprints/VRPawn.ActiveText Bar` (`self.VRPawn`) (`|GetArrayItem` (`self.Text`) (`self.TextIndex`)) (`self.Chars Per Second`)))
      (if _iswrite
        (`KismetSystemLibrary.PrintString` (`KismetStringLibrary.Concat_StrStr` (`KismetStringLibrary.Conv_IntToString` _textindex) (`KismetStringLibrary.Conv_BoolToString` _iswrite)) false)
        (set `self.TextIndex` (+ (`self.TextIndex`) 1)))
      (else
        (`KismetSystemLibrary.PrintString` "Destory" false)
        (set `/Game/VRTemplate/Blueprints/VRPawn.CanTeleport` true (`self.VRPawn`))
        (`self.K2_DestroyActor`)))))

(event `self.Box.OnComponentBeginOverlap`
  (params (OverlappedComponent :type "PrimitiveComponent Object Reference") (OtherActor :type "Actor Object Reference") (OtherComp :type "PrimitiveComponent Object Reference") (OtherBodyIndex :type Integer) (bFromSweep :type Boolean) (SweepResult :type "HitResult Structure (by ref)"))
  (if (not (`self.StartPlay`))
    (bind _asvrpawn (cast `/Game/VRTemplate/Blueprints/VRPawn` (`self.GetParentActor` OtherActor)))
    (set `self.VRPawn` _asvrpawn)
    (set `self.IsPlayerOn` true)
    (set `/Game/VRTemplate/Blueprints/VRPawn.CanTeleport` false _asvrpawn)))

(event `self.Box.OnComponentEndOverlap`
  (params (OverlappedComponent :type "PrimitiveComponent Object Reference") (OtherActor :type "Actor Object Reference") (OtherComp :type "PrimitiveComponent Object Reference") (OtherBodyIndex :type Integer))
  (if (== OtherActor (stale `self.Box.OnComponentBeginOverlap` OtherActor))
    (set `self.IsPlayerOn` false)))

(event `self.ReceiveBeginPlay`
  (if (`self.StartPlay`)
    (`KismetSystemLibrary.Delay` (`self.StartPlayDelay`))
    (`self.Start`)))

(event `Start`
  (bind _asvrpawn (cast `/Game/VRTemplate/Blueprints/VRPawn` (`GameplayStatics.GetPlayerPawn` 0) :!pure true))
  (set `self.VRPawn` _asvrpawn)
  (set `/Game/VRTemplate/Blueprints/VRPawn.CanTeleport` false _asvrpawn)
  (set `self.IsPlayerOn` true))

(fn `UserConstructionScript`)