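; BP_TypewriterWidget is an actor with a widget component that shows typewriter-style text through a TypewriterWidget.
; It acts as a wrapper, casting the component's user widget to forward message writing at a given characters-per-second rate, removal and an IsRemoved query.
; Failed casts in write and remove print error strings, and BeginPlay enables input from the first player controller.
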(event `self.ReceiveBeginPlay`
  ;[1 1 1] Begin Play
  (`self.EnableInput` (`GameplayStatics.GetPlayerController` 0)))

(fn `GetIsRemoved`
  (returns (IsRemoved :type Boolean))
  (return (`/Game/Text/TypewriterWidget.IsRemoved` (cast `/Game/Text/TypewriterWidget` (`WidgetComponent.GetUserWidgetObject` (`self.Widget`)) :!pure true))))

(fn `RemoveMessage`
  (bind (_astypewriter_widget _bsuccess) (cast `/Game/Text/TypewriterWidget` (`WidgetComponent.GetUserWidgetObject` (`self.Widget`)) :!pure true))
  (if _bsuccess
    (`/Game/Text/TypewriterWidget.Remove` _astypewriter_widget)
    (else
      (`KismetSystemLibrary.PrintString` "TYpewriterWidget Remove Error"))))

(fn `UserConstructionScript`)

(fn `Write Message`
  (params (Text :type String) (CharsPerSecond :type "Float (double-precision)" :default 0.0))
  (returns (IsWrite :type Boolean))
  (bind (_astypewriter_widget _bsuccess) (cast `/Game/Text/TypewriterWidget` (`WidgetComponent.GetUserWidgetObject` (`self.Widget`)) :!pure true))
  (if _bsuccess
    (bind _canwrite (`/Game/Text/TypewriterWidget.WriteFunc` _astypewriter_widget Text CharsPerSecond))
    (return _canwrite)
    (else
      (`KismetSystemLibrary.PrintString` "TYpewriterWidgetError"))))